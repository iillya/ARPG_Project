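; Anim notify state that closes out a montage action by releasing the owner's action state and resetting its combo.
; On begin, it removes the OtherAction state gameplay tag locally and stops the active montage if the owning Character has non-zero movement acceleration, letting movement cut the animation short.
; The acceleration check runs only once, at window start.
; On end, it sends the reset-combo interface message to the owner.
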(fn ReceivedNotifyBegin
  (params (MeshComp :type Skeletal%20Mesh%20Component%20Object%20Reference) (Animation :type Anim%20Sequence%20Base%20Object%20Reference) (TotalDuration :type Float%20%28single-precision%29) (EventReference :type Anim%20Notify%20Event%20Reference%20Structure%20%28by%20ref%29))
  (bind _returnvalue (Components|GetOwner MeshComp))
  (Ability|GameplayEffect|RemoveLooseGameplayTags _returnvalue (GameplayTags|MakeLiteralGameplayTagContainer "(GameplayTags=((TagName=\"Charactar.State.Action.OtherAction\"),(TagName=\"Charactar.State.Action.Jumping\"),(TagName=\"Charactar.State.Action.Attacking\"),(TagName=\"Charactar.State.Action.Rolling\")))"))
  (bind _as角色 (Utilities|Casting|CastToCharacter _returnvalue))
  (Utilities|IsValid _as角色
    (:Is%20Valid
      (if (!= (Math|Vector|VectorLength (Pawn|Components|CharacterMovement|GetCurrentAcceleration (Variables|/Script/Engine.Character|GetCharacterMovement _as角色))) 0.0)
        (Animation|StopAnimMontage _as角色 (Animation|Montage|GetCurrentActiveMontage (Components|SkeletalMesh|GetAnimInstance MeshComp)))
        (return false)))))

(fn ReceivedNotifyEnd
  (params (MeshComp :type Skeletal%20Mesh%20Component%20Object%20Reference) (Animation :type Anim%20Sequence%20Base%20Object%20Reference) (EventReference :type Anim%20Notify%20Event%20Reference%20Structure%20%28by%20ref%29))
  (Class|BPICharacter|INTResetCombo(Message) (Components|GetOwner MeshComp))
  (return false))